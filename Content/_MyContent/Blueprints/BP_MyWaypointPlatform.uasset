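; Moving platform actor that travels along an array of placed waypoint actors, with Start and Stop functions to control it.
; BeginPlay hides each waypoint and calls PlatformStart inside that loop, which resets to the first segment and plays MotionTimeline at the set Rate.
; The timeline lerps relative location between waypoint world positions; its event advances segments, restarting from the first if Loop is set.
; Construction script applies the configurable mesh and material.
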(event `PlatformStart`
  (`self.SetFirstWaypoint`)
  (`TimelineComponent.SetPlayRate` (`self.Motion Timeline`) (`self.Rate`))
  (`TimelineComponent.PlayFromStart` (`self.Motion Timeline`)))

(event `self.ReceiveBeginPlay`
  (for _array_element (`self.Waypoints`)
    (`self.SetActorHiddenInGame` _array_element true)
    (`self.PlatformStart`)))

(fn `PathIsFinished`
  (returns (IsFinished :type Boolean))
  (return (== (`self.NextWaypointIndex`) (- (`KismetArrayLibrary.Array_Length` (`self.Waypoints`)) 1))))

(fn `SetFirstWaypoint`
  (set `self.CurrentWaypointIndex` 0)
  (set `self.NextWaypointIndex` 1)
  (`self.SetPositions`))

(fn `SetNextWaypoint`
  (bind _result (`/Engine/EditorBlueprintResources/StandardMacros.IncrementInt` (`self.CurrentWaypointIndex`))
    (:`  `
      (set `self.NextWaypointIndex` (+ _result 1))
      (`self.SetPositions`))))

(fn `SetPositions`
  (bind _waypoints (`self.Waypoints`))
  (set `self.CurrentWaypointPosition` (`self.K2_GetActorLocation` (`|GetArrayItem` _waypoints (`self.CurrentWaypointIndex`))))
  (set `self.NextWaypointPosition` (`self.K2_GetActorLocation` (`|GetArrayItem` _waypoints (`self.NextWaypointIndex`)))))

(fn `Start`
  (`self.PlatformStart`))

(fn `Stop`
  (`TimelineComponent.Stop` (`self.Motion Timeline`)))

(fn `UserConstructionScript`
  (`StaticMeshComponent.SetStaticMesh` (`self.PlatformMesh`) (`self.StaticMesh`))
  (`PrimitiveComponent.SetMaterial` (`self.PlatformMesh`) 0 (`self.Material`)))