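; A destructible mesh obstacle that advances toward the player and can be shattered by projectiles.
; While the game manager's trigger flag is set, Tick moves it a fixed step along world X, with no delta-time scaling.
; A box overlap with BP_Projectile applies radius damage, enables gravity, removes the box and destroys the actor after a short delay.
; An overlap with ThirdPersonCharacter instead changes the game manager's state.
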(event `self.ReceiveTick`
  (params (DeltaSeconds :type "Float (single-precision)"))
  ;[1 1 1] MovementTowardsPlayer
  (bind _mygamemanager (`/Game/_MyContent/Blueprints/BP_FunctionLibrary.GetMyGameManager`))
  (if (`/Game/_MyContent/Blueprints/BP_MyGameManager.DestructableMeshTrigger` _mygamemanager)
    (`self.K2_SetActorLocation` (+ (`SceneComponent.K2_GetComponentLocation` (`self.Destructible`)) (8.0 0.0 0.0)))))

(event `self.Box.OnComponentBeginOverlap`
  (params (OverlappedComponent :type "PrimitiveComponent Object Reference") (OtherActor :type "Actor Object Reference") (OtherComp :type "PrimitiveComponent Object Reference") (OtherBodyIndex :type Integer) (bFromSweep :type Boolean) (SweepResult :type "HitResult Structure (by ref)"))
  (bind _returnvalue (`GameplayStatics.GetObjectClass` OtherActor))
  (bind _destructible (`self.Destructible`))
  ;[1 1 1] MeshDestruction
  (if (== _returnvalue "/Game/_MyContent/Blueprints/BP_Projectile.BP_Projectile_C")
    (`DestructibleComponent.ApplyRadiusDamage` _destructible 20.0 (`SceneComponent.K2_GetComponentLocation` _destructible) 20.0 0.0 false)
    (`PrimitiveComponent.SetEnableGravity` (`self.Destructible`) true)
    (`ActorComponent.K2_DestroyComponent` (`self.Box`))
    (`KismetSystemLibrary.Delay` 2.0)
    (`self.K2_DestroyActor`)
    (elif (== _returnvalue "/Game/ThirdPersonBP/Blueprints/ThirdPersonCharacter.ThirdPersonCharacter_C")
      (bind _mygamemanager (`/Game/_MyContent/Blueprints/BP_FunctionLibrary.GetMyGameManager`))
      (`/Game/_MyContent/Blueprints/BP_MyGameManager.SetState` _mygamemanager "NewEnumerator2"))))

(fn `UserConstructionScript`)