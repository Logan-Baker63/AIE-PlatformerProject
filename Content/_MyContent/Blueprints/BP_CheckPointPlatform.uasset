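; BP_CheckPointPlatform is a one-time checkpoint platform that saves the player's position as the spawn point.
; When the player first overlaps its box, it sets a checkpointed flag and moves the Spawn actor to the player's location.
; It then hides the UI, shows a W_Checkpoint widget with a sound, and after a short delay hides the UI again and restores the HUD through the game manager.
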(event `self.ReceiveBeginPlay`
  (set `self.IsCheckpointed` false))

(event `self.Box.OnComponentBeginOverlap`
  (params (OverlappedComponent :type "PrimitiveComponent Object Reference") (OtherActor :type "Actor Object Reference") (OtherComp :type "PrimitiveComponent Object Reference") (OtherBodyIndex :type Integer) (bFromSweep :type Boolean) (SweepResult :type "HitResult Structure (by ref)"))
  (bind _player (`self.Player`))
  (if (== OtherActor _player)
    (if (not (`self.IsCheckpointed`))
      (set `self.IsCheckpointed` true)
      (`self.K2_SetActorLocation` (`self.Spawn`) (`self.K2_GetActorLocation` _player) false false)
      (`/Game/_MyContent/Blueprints/BP_FunctionLibrary.HideUI`)
      (bind _returnvalue (`|CreateWidget` "/Game/_MyContent/UI/W_Checkpoint.W_Checkpoint_C"))
      (`UserWidget.AddToViewport` _returnvalue 0)
      (`GameplayStatics.PlaySoundAtLocation` "/Game/_MyContent/Audio/CheckpointNoise_Cue.CheckpointNoise_Cue" (0.0 0.0 0.0) (struct) 1.0 1.0 0.0 null null null)
      (`KismetSystemLibrary.Delay` 1.5)
      (`/Game/_MyContent/Blueprints/BP_FunctionLibrary.HideUI`)
      (bind _mygamemanager (`/Game/_MyContent/Blueprints/BP_FunctionLibrary.GetMyGameManager`))
      (`/Game/_MyContent/Blueprints/BP_MyGameManager.ShowHUD` _mygamemanager true))))

(fn `UserConstructionScript`)