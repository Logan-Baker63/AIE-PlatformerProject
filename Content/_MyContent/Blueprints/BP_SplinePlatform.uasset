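; BP_SplinePlatform is a platform actor that moves its mesh along a spline, starting on BeginPlay.
; A timeline's SplineDistance track, scaled by spline length, sets the mesh's world location each update without sweeping or changing rotation.
; When the timeline finishes it replays from the start, so the motion loops indefinitely.
; The Construction Script applies the mesh and material from variables.
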(event `self.ReceiveBeginPlay`
  (`self.PlatformStart`))

(event `PlatformStart`
  (bind (_direction _splinedistance) (`Timeline|MotionTimeline` :!via `PlayFromStart` :!label _label)
    (:`Update`
      (`SceneComponent.K2_SetWorldLocation` (`self.PlatformMesh`) (`SplineComponent.GetLocationAtDistanceAlongSpline` (`self.Spline`) (* _splinedistance (`SplineComponent.GetSplineLength` (`self.Spline`))) "World") false false))
    (:`Finished`
      (if true
        (goto _label :!via `PlayFromStart`)))))

(fn `UserConstructionScript`
  (bind _platformmesh (`self.PlatformMesh`))
  (`StaticMeshComponent.SetStaticMesh` _platformmesh (`self.StaticMesh`))
  (`PrimitiveComponent.SetMaterial` _platformmesh 0 (`self.Material`)))