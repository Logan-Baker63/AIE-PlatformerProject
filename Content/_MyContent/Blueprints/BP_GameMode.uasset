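; BP_GameMode is a game mode Blueprint that locates the game manager and provides setup for the game's UI.
; On BeginPlay it stores the first BP_MyGameManager found in the level as GameManager.
; CreateUI builds the abandon, lost, won and health widgets, stores each on the manager returned by GetMyGameManager and adds them all to the viewport.
; Nothing in this Blueprint calls CreateUI.
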(event `self.ReceiveBeginPlay`
  (bind _outactors (`GameplayStatics.GetAllActorsOfClass` "/Game/_MyContent/Blueprints/BP_MyGameManager.BP_MyGameManager_C"))
  (set `self.GameManager` (`|GetArrayItem` _outactors)))

(fn `CreateUI`
  (bind _mygamemanager (`/Game/_MyContent/Blueprints/BP_FunctionLibrary.GetMyGameManager`))
  (bind _returnvalue (`|CreateWidget` "/Game/_MyContent/UI/W_Abandon.W_Abandon_C"))
  (bind _output_get (set `/Game/_MyContent/Blueprints/BP_MyGameManager.WidgetAbandon` _returnvalue _mygamemanager))
  (`UserWidget.AddToViewport` _output_get 0)
  (bind _returnvalue_2 (`|CreateWidget` "/Game/_MyContent/UI/W_Lost.W_Lost_C"))
  (bind _output_get_2 (set `/Game/_MyContent/Blueprints/BP_MyGameManager.WidgetLost` _returnvalue_2 _mygamemanager))
  (`UserWidget.AddToViewport` _output_get_2 0)
  (bind _returnvalue_3 (`|CreateWidget` "/Game/_MyContent/UI/W_Won.W_Won_C"))
  (bind _output_get_3 (set `/Game/_MyContent/Blueprints/BP_MyGameManager.WidgetWon` _returnvalue_3 _mygamemanager))
  (`UserWidget.AddToViewport` _output_get_3 0)
  (bind _returnvalue_4 (`|CreateWidget` "/Game/_MyContent/UI/W_Health.W_Health_C"))
  (bind _output_get_4 (set `/Game/_MyContent/Blueprints/BP_MyGameManager.WidgetHealth` _returnvalue_4 _mygamemanager))
  (`UserWidget.AddToViewport` _output_get_4 0))

(fn `UserConstructionScript`)