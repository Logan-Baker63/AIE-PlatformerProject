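; BP_MyGameManager is an actor that manages the game's state, switching between Running and Abandon.
; Init has BP_GameMode create the UI, then requests the Running state.
; SetState ignores repeated states, otherwise hides the UI and applies the new one: Running hides the mouse and unpauses, Abandon shows the abandon widget and mouse and pauses.
; GetState exposes the current state, and the event graph holds no active logic.
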(fn `GetState`
  (returns (State :type "/Game/_MyContent/Blueprints/MyGameStates Enum"))
  (return (`self.CurrentGameState`)))

(fn `Init`
  (bind _asbp_game_mode (cast `/Game/_MyContent/Blueprints/BP_GameMode` (`GameplayStatics.GetGameMode`)))
  (`/Game/_MyContent/Blueprints/BP_GameMode.CreateUI` _asbp_game_mode)
  (`self.SetState` "NewEnumerator0"))

(fn `SetState`
  (params (`New State` :type "/Game/_MyContent/Blueprints/MyGameStates Enum" :default "NewEnumerator0"))
  (if (!= `New State` (`self.CurrentGameState`))
    (`/Game/_MyContent/Blueprints/BP_FunctionLibrary.HideUI`)
    (bind _output_get (set `self.CurrentGameState` `New State`))
    (switch `/Game/_MyContent/Blueprints/MyGameStates` _output_get
      (:`NewEnumerator0`
        (`/Game/_MyContent/Blueprints/BP_FunctionLibrary.ShowMouse` false)
        (`GameplayStatics.SetGamePaused` false))
      (:`NewEnumerator3`
        (`Widget.SetVisibility` (`self.WidgetAbandon`) "Visible")
        (`/Game/_MyContent/Blueprints/BP_FunctionLibrary.ShowMouse` true)
        (`GameplayStatics.SetGamePaused` true)))))

(fn `UserConstructionScript`)