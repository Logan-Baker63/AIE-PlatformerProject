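; BP_CheckpointReinforcer is a trigger volume that enforces Level 1 coin collection before the player can progress past it.
; When a ThirdPersonCharacter overlaps the Box while the game manager's Level1CoinCollected is false, it moves the player to a hard-coded location.
; It then swaps the current UI for a W_CoinsRequired notice and, after a short delay, hides it and restores the HUD through the game manager.
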(event `self.Box.OnComponentBeginOverlap`
  (params (OverlappedComponent :type "PrimitiveComponent Object Reference") (OtherActor :type "Actor Object Reference") (OtherComp :type "PrimitiveComponent Object Reference") (OtherBodyIndex :type Integer) (bFromSweep :type Boolean) (SweepResult :type "HitResult Structure (by ref)"))
  (if (== (`GameplayStatics.GetObjectClass` OtherActor) "/Game/ThirdPersonBP/Blueprints/ThirdPersonCharacter.ThirdPersonCharacter_C")
    (bind _mygamemanager (`/Game/_MyContent/Blueprints/BP_FunctionLibrary.GetMyGameManager`))
    (if (not (`/Game/_MyContent/Blueprints/BP_MyGameManager.Level1CoinCollected` _mygamemanager))
      (`self.K2_SetActorLocation` (`self.Player`) (1610.0 2210.0 750.0) false false)
      (`/Game/_MyContent/Blueprints/BP_FunctionLibrary.HideUI`)
      (bind _returnvalue (`|CreateWidget` "/Game/_MyContent/UI/W_CoinsRequired.W_CoinsRequired_C"))
      (`UserWidget.AddToViewport` _returnvalue 0)
      (`KismetSystemLibrary.Delay` 1.5)
      (`/Game/_MyContent/Blueprints/BP_FunctionLibrary.HideUI`)
      (bind _mygamemanager_2 (`/Game/_MyContent/Blueprints/BP_FunctionLibrary.GetMyGameManager`))
      (`/Game/_MyContent/Blueprints/BP_MyGameManager.ShowHUD` _mygamemanager_2 true))))

(fn `UserConstructionScript`)