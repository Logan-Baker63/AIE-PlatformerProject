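; BP_JetpackPickup is a spinning collectible that grants the player character the jetpack on overlap.
; Tick rotates the cube, and the box overlap sets JetpackIsCollected on player 0's ThirdPersonCharacter, destroys the pickup and teleport-free moves BlockingWall to a hardcoded location.
; It then hides UI, shows a collected widget and, after a short Delay, restores the HUD through the game manager.
; That UI sequence follows DestroyActor and is marked broken.
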(event `self.ReceiveTick`
  (params (DeltaSeconds :type "Float (single-precision)"))
  (`SceneComponent.K2_AddLocalRotation` (`self.Cube`) (struct :`Yaw` 1.0) false false))

(event `self.Box.OnComponentBeginOverlap`
  (params (OverlappedComponent :type "PrimitiveComponent Object Reference") (OtherActor :type "Actor Object Reference") (OtherComp :type "PrimitiveComponent Object Reference") (OtherBodyIndex :type Integer) (bFromSweep :type Boolean) (SweepResult :type "HitResult Structure (by ref)"))
  (if (== (`GameplayStatics.GetObjectClass` OtherActor) "/Game/ThirdPersonBP/Blueprints/ThirdPersonCharacter.ThirdPersonCharacter_C")
    (bind _asthird_person_character (cast `/Game/ThirdPersonBP/Blueprints/ThirdPersonCharacter` (`GameplayStatics.GetPlayerCharacter` 0)))
    (set `/Game/ThirdPersonBP/Blueprints/ThirdPersonCharacter.JetpackIsCollected` true _asthird_person_character)
    (`self.K2_DestroyActor`)
    (`self.K2_SetActorLocation` (`self.BlockingWall`) (4872.660156 8827.070312 654.0) false false)
    ;[1 1 1] Broken Somehow
    (`/Game/_MyContent/Blueprints/BP_FunctionLibrary.HideUI`)
    (bind _returnvalue (`|CreateWidget` "/Game/_MyContent/UI/W_JetpackCollected.W_JetpackCollected_C"))
    (`UserWidget.AddToViewport` _returnvalue 0)
    (`KismetSystemLibrary.Delay` 0.2)
    (`/Game/_MyContent/Blueprints/BP_FunctionLibrary.HideUI`)
    (bind _mygamemanager (`/Game/_MyContent/Blueprints/BP_FunctionLibrary.GetMyGameManager`))
    (`/Game/_MyContent/Blueprints/BP_MyGameManager.ShowHUD` _mygamemanager true)
    (`KismetSystemLibrary.PrintString` "Hello")))

(fn `UserConstructionScript`)