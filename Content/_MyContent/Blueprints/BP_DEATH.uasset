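; BP_DEATH is a rising lava hazard that changes the game state when the player touches it.
; A Delay on Tick, timed by RisingSpeed, paces teleport-free, unswept moves to the Lava actor's location plus RisingDistance, so the value acts as an interval between steps.
; Its static mesh's begin overlap checks for the player, then sets a new state on the game manager.
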(event `self.ReceiveTick`
  (params (DeltaSeconds :type "Float (single-precision)"))
  (`KismetSystemLibrary.Delay` (`self.RisingSpeed`))
  (`self.K2_SetActorLocation` (+ (`self.Rising distance`) (`self.K2_GetActorLocation` (`self.Lava`)))))

(event `self.StaticMeshComponent.OnComponentBeginOverlap`
  (params (OverlappedComponent :type "PrimitiveComponent Object Reference") (OtherActor :type "Actor Object Reference") (OtherComp :type "PrimitiveComponent Object Reference") (OtherBodyIndex :type Integer) (bFromSweep :type Boolean) (SweepResult :type "HitResult Structure (by ref)"))
  (if (== OtherActor (`self.Player`))
    (bind _mygamemanager (`/Game/_MyContent/Blueprints/BP_FunctionLibrary.GetMyGameManager`))
    (`/Game/_MyContent/Blueprints/BP_MyGameManager.SetState` _mygamemanager "NewEnumerator2")))

(fn `UserConstructionScript`)