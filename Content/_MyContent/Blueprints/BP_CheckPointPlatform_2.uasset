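; BP_CheckPointPlatform_2 is a one-time checkpoint platform that activates only if the game manager's Level1CoinCollected flag is set.
; When the player overlaps its box, it moves the Spawn actor to the player's location, shows a checkpoint widget and plays a sound at world origin.
; Without the flag, it shows a coins-required widget instead.
; Either message clears after a short delay, then the game manager restores the HUD.
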(event `self.ReceiveBeginPlay`
  (set `self.IsCheckpointed` false))

(event `self.Box.OnComponentBeginOverlap`
  (params (OverlappedComponent :type "PrimitiveComponent Object Reference") (OtherActor :type "Actor Object Reference") (OtherComp :type "PrimitiveComponent Object Reference") (OtherBodyIndex :type Integer) (bFromSweep :type Boolean) (SweepResult :type "HitResult Structure (by ref)"))
  (if (== OtherActor (`self.Player`))
    (if (not (`self.IsCheckpointed`))
      (bind _mygamemanager (`/Game/_MyContent/Blueprints/BP_FunctionLibrary.GetMyGameManager`))
      (if (`/Game/_MyContent/Blueprints/BP_MyGameManager.Level1CoinCollected` _mygamemanager)
        (set `self.IsCheckpointed` true)
        (`self.K2_SetActorLocation` (`self.Spawn`) (`self.K2_GetActorLocation` (`self.Player`)) false false)
        (`/Game/_MyContent/Blueprints/BP_FunctionLibrary.HideUI`)
        (bind _returnvalue (`|CreateWidget` "/Game/_MyContent/UI/W_Checkpoint.W_Checkpoint_C"))
        (`UserWidget.AddToViewport` _returnvalue 0)
        (`GameplayStatics.PlaySoundAtLocation` "/Game/_MyContent/Audio/CheckpointNoise_Cue.CheckpointNoise_Cue" (0.0 0.0 0.0) (struct) 1.0 1.0 0.0 null null null)
        (`KismetSystemLibrary.Delay` 1.5)
        (`/Game/_MyContent/Blueprints/BP_FunctionLibrary.HideUI`)
        (bind _mygamemanager_2 (`/Game/_MyContent/Blueprints/BP_FunctionLibrary.GetMyGameManager`))
        (`/Game/_MyContent/Blueprints/BP_MyGameManager.ShowHUD` _mygamemanager_2 true)
        (else
          (`/Game/_MyContent/Blueprints/BP_FunctionLibrary.HideUI`)
          (bind _returnvalue_2 (`|CreateWidget` "/Game/_MyContent/UI/W_CoinsRequired.W_CoinsRequired_C"))
          (`UserWidget.AddToViewport` _returnvalue_2 0)
          (`KismetSystemLibrary.Delay` 1.5)
          (`/Game/_MyContent/Blueprints/BP_FunctionLibrary.HideUI`)
          (bind _mygamemanager_3 (`/Game/_MyContent/Blueprints/BP_FunctionLibrary.GetMyGameManager`))
          (`/Game/_MyContent/Blueprints/BP_MyGameManager.ShowHUD` _mygamemanager_3 true))))))

(fn `UserConstructionScript`)